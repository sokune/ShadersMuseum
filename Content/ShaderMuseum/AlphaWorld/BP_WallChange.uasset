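; BP_WallChange toggles the material on a set of wall meshes in the AlphaWorld area of the shader museum.
; ChangeWall loops over the Walls array, setting material slot 0 to M_Walls or M_Black based on IsOn, then flips that flag.
; It has no active event logic of its own, so the swap runs only when ChangeWall is called.
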(fn `ChangeWall`
  (for _array_element (`self.Walls`)
    (`PrimitiveComponent.SetMaterial` (`StaticMeshActor.StaticMeshComponent` _array_element) 0 (select `bool` (`self.IsOn`) :`false` "/Game/ShaderMuseum/AlphaWorld/M_Black.M_Black" :`true` "/Game/ShaderMuseum/Architectures/M_Walls.M_Walls" :!type "MaterialInterface Object Reference")))
  (set `self.IsOn` (not (`self.IsOn`))))

(fn `UserConstructionScript`
  (`parent.UserConstructionScript`))