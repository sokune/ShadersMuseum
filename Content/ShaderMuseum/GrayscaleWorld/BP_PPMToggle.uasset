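; Shader museum toggle actor that switches the black-and-white and dithering post process effects on and off.
; Each toggle function flips a volume's BlendWeight between 0 and 1, finding it by display name among PostProcessVolumes on first use and caching it.
; Both functions share one cached PPBlackNWhite reference and IsOff flag, with inverted weights in the dithering toggle, so whichever volume is cached first serves both.
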(fn `ToggleBlackNWhitePPM`
  (bind _pp_blacknwhite (`self.PP_BlackNWhite`))
  (`/Engine/EditorBlueprintResources/StandardMacros.IsValid` (`self.PP_BlackNWhite`)
    (:`Is Valid`
      _)
    (:`Is Not Valid`
      (bind _outactors (`GameplayStatics.GetAllActorsOfClass` "/Script/Engine.PostProcessVolume"))
      (for _array_element _outactors
        (if (`KismetStringLibrary.EqualEqual_StrStr` (`KismetSystemLibrary.GetDisplayName` _array_element) "PP_BlackNWhite")
          (set `self.PP_BlackNWhite` _array_element)
          (break)))))
  (if (`self.IsOff`)
    (set `PostProcessVolume.BlendWeight` 1.0 _pp_blacknwhite)
    (set `self.IsOff` false)
    (else
      (set `PostProcessVolume.BlendWeight` 0.0 _pp_blacknwhite)
      (set `self.IsOff` true))))

(fn `ToggleDitheringPPM`
  (bind _pp_blacknwhite (`self.PP_BlackNWhite`))
  (`/Engine/EditorBlueprintResources/StandardMacros.IsValid` (`self.PP_BlackNWhite`)
    (:`Is Valid`
      _)
    (:`Is Not Valid`
      (bind _outactors (`GameplayStatics.GetAllActorsOfClass` "/Script/Engine.PostProcessVolume"))
      (for _array_element _outactors
        (if (`KismetStringLibrary.EqualEqual_StrStr` (`KismetSystemLibrary.GetDisplayName` _array_element) "PP_Dithering")
          (set `self.PP_BlackNWhite` _array_element)
          (break)))))
  (if (`self.IsOff`)
    (set `PostProcessVolume.BlendWeight` 0.0 _pp_blacknwhite)
    (set `self.IsOff` false)
    (else
      (set `PostProcessVolume.BlendWeight` 1.0 _pp_blacknwhite)
      (set `self.IsOff` true))))

(fn `UserConstructionScript`
  (`parent.UserConstructionScript`))